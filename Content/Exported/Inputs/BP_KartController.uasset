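; BP_KartController is the player controller for a kart racing game, handling race start, end and UI.
; BeginPlay adds the input mapping and shows the in-game HUD, or in debug sets the kart pawn racing immediately.
; GameStart enables racing and plays a Timeline that Tick copies into Timer.
; GameOver stops the timer and swaps to the game-over widget, after which Enter opens BowsersCastle.
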(event `self.ReceiveBeginPlay`
  (`EnhancedInputSubsystemInterface.AddMappingContext` (subsystem `EnhancedInputLocalPlayerSubsystem`) "/Game/Exported/Inputs/IMC_MarioKart.IMC_MarioKart" 0 (struct))
  (if (`self.Debug`)
    (bind _asbp_tanooki_kart_pawn (cast `/Game/Exported/TanookiKart/Blueprints/BP_TanookiKart_Pawn` (`self.K2_GetPawn`)))
    (set `/Game/Exported/TanookiKart/Blueprints/BP_TanookiKart_Pawn.IsRacing` true _asbp_tanooki_kart_pawn)
    (else
      (bind _returnvalue (`|CreateWidget` "/Game/UI/InGame/WBP_InGame.WBP_InGame_C" self))
      (bind _output_get (set `self.InGameUI` _returnvalue))
      (`UserWidget.AddToViewport` _output_get 0))))

(event `self.ReceiveTick`
  (params (DeltaSeconds :type "Float (single-precision)"))
  (if (`self.HasRaceStarted`)
    (set `self.Timer` (stale `GameStart` _timer))))

(event `GameStart`
  (bind _asbp_tanooki_kart_pawn (cast `/Game/Exported/TanookiKart/Blueprints/BP_TanookiKart_Pawn` (`self.K2_GetPawn`)))
  (set `/Game/Exported/TanookiKart/Blueprints/BP_TanookiKart_Pawn.IsRacing` true _asbp_tanooki_kart_pawn)
  (set `self.HasRaceStarted` true)
  (bind (_direction _timer) (`Timeline|Timeline` :!label _label)))

(event `GameOver`
  (set `self.HasRaceStarted` false)
  (`Widget.RemoveFromParent` (`self.InGameUI`))
  (bind _returnvalue (`|CreateWidget` "/Game/UI/EndGame/WBP_GameOver.WBP_GameOver_C" self))
  (`UserWidget.AddToViewport` _returnvalue 0)
  (set `self.IsGameEnded` true)
  (goto _label :!via `Stop`))

(event `Key|Enter`
  (params (Key :type "Key Structure"))
  (:`Pressed`
    (if (`self.IsGameEnded`)
      (`GameplayStatics.OpenLevelBySoftObjectPtr` "/Game/Level/BowsersCastle.BowsersCastle"))))

(fn `UserConstructionScript`)