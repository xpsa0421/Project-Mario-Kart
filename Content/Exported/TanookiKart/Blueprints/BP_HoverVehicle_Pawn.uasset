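; Player-driven kart pawn with Mario Kart-style drifting, mini-jump, horn and chase/rear camera toggle.
; Enhanced Input feeds target speeds to a movement component, while Tick derives grounded state from four hover components and animates wheel steering and spin.
; Drift hold time sets three colored spark tiers; releasing triggers a matching timed boost with particles and FOV timelines.
; Boost-panel overlaps only print debug text.
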(event `self.ReceiveTick`
  (params (DeltaSeconds :type "Float (single-precision)"))
  ;[1 1 1] Alter Kart Wheel Animation and Status
  (`self.CheckIfGrounded`)
  (`self.Set Steering Angle`)
  (`self.Set Wheel Rotation`))

(event `self.ReceiveBeginPlay`
  ;[1 1 1 1 30] Initial Settings
  (`|ExecutionSequence`
    (:`then_0`
      ;;[1 1 1] Set Input Mapping Context
      (bind _asplayer_controller (cast `PlayerController` (`self.GetController`)))
      (bind _returnvalue (pcsubsystem `EnhancedInputLocalPlayerSubsystem` _asplayer_controller))
      (`/Engine/EditorBlueprintResources/StandardMacros.IsValid` _returnvalue
        (:`Is Valid`
          (`EnhancedInputSubsystemInterface.AddMappingContext` _returnvalue "/Game/Exported/Inputs/IMC_MarioKart.IMC_MarioKart" 0 (struct)))))
    (:`then_1`
      ;;[1 1 1] Initialise Particle System Parameters
      (`FXSystemComponent.SetIntParameter` (`self.SmokeParticle_L`) "ParticleCount" 100)
      (`FXSystemComponent.SetIntParameter` (`self.SmokeParticle_R`) "ParticleCount" 100)
      (`FXSystemComponent.SetIntParameter` (`self.DriftSmokeParticle_L`) "ParticleCount" 10000)
      (`FXSystemComponent.SetIntParameter` (`self.DriftSmokeParticle_R`) "ParticleCount" 10000))
    (:`then_2`
      ;;[1 1 1] Set Default Camera
      (`ActorComponent.SetActive` (`self.ChaseCamera`) true false)
      (`ActorComponent.SetActive` (`self.RearCamera`) false false))))

(event `EnhancedInput|/Game/Exported/Inputs/Actions/IA_Throttle`
  (params (ActionValue :type "Float (double-precision)") (ElapsedSeconds :type "Float (double-precision)") (TriggeredSeconds :type "Float (double-precision)") (InputAction :type "InputAction Object Reference" :default "/Game/Exported/Inputs/Actions/IA_Throttle.IA_Throttle"))
  ;[1 1 1 1 30] Handle Inputs
  ;;[1 1 1] Handle Input Throttle
  (:`Triggered`
    (if (`self.IsGrounded`) :!label _label
      (set `/Game/Exported/TanookiKart/Blueprints/BP_MovementComponent.TargetSpeed` (* ActionValue (`self.DefaultSpeedMultiplier`) (`self.BoostMultiplier`)) (`self.MovementComponent`))))
  (:`Completed`
    (goto _label)))

(event `EnhancedInput|/Game/Exported/Inputs/Actions/IA_Horn`
  (params (ActionValue :type Boolean) (ElapsedSeconds :type "Float (double-precision)") (TriggeredSeconds :type "Float (double-precision)") (InputAction :type "InputAction Object Reference" :default "/Game/Exported/Inputs/Actions/IA_Horn.IA_Horn"))
  ;[1 1 1 1 30] Handle Inputs
  ;;[1 1 1] Handle Input Horn
  (:`Triggered`
    (if (not (`self.HornPlaying`))
      (set `self.HornPlaying` true)
      (`GameplayStatics.PlaySoundAtLocation` "/Game/Exported/Sounds/Karts/WAV_Tnk_Horn.WAV_Tnk_Horn" (`self.K2_GetActorLocation`) (struct) 1.0 1.0 0.0 null null null null)
      (`KismetSystemLibrary.Delay` 0.531)
      (set `self.HornPlaying` false))))

(event `EnhancedInput|/Game/Exported/Inputs/Actions/IA_Steer`
  (params (ActionValue :type "Float (double-precision)") (ElapsedSeconds :type "Float (double-precision)") (TriggeredSeconds :type "Float (double-precision)") (InputAction :type "InputAction Object Reference" :default "/Game/Exported/Inputs/Actions/IA_Steer.IA_Steer"))
  (bind _returnvalue (`|GetInputActionValue`))
  ;[1 1 1 1 30] Handle Inputs
  ;;[1 1 1] Handle Input Steer
  (:`Triggered`
    (if (not (`self.IsDrifting`)) :!label _label_2
      (set `/Game/Exported/TanookiKart/Blueprints/BP_MovementComponent.TargetAngularSpeed` (* ActionValue 100.0 (select `bool` (== _returnvalue 0.0) :`false` _returnvalue :`true` 1.0)) (`self.MovementComponent`))))
  (:`Completed`
    (goto _label_2)))

(event `EnhancedInput|/Game/Exported/Inputs/Actions/IA_ToggleCamera`
  (params (ActionValue :type Boolean) (ElapsedSeconds :type "Float (double-precision)") (TriggeredSeconds :type "Float (double-precision)") (InputAction :type "InputAction Object Reference" :default "/Game/Exported/Inputs/Actions/IA_ToggleCamera.IA_ToggleCamera"))
  ;[1 1 1 1 30] Handle Inputs
  ;;[1 1 1] Handle Input Toggle Camera
  (:`Triggered`
    (`/Engine/EditorBlueprintResources/StandardMacros.FlipFlop`
      (:`A`
        (`ActorComponent.SetActive` (`self.ChaseCamera`) false false)
        (`ActorComponent.SetActive` (`self.RearCamera`) true false))
      (:`B`
        (`ActorComponent.SetActive` (`self.ChaseCamera`) true false)
        (`ActorComponent.SetActive` (`self.RearCamera`) false false)))))

(event `EnhancedInput|/Game/Exported/Inputs/Actions/IA_Drift`
  (params (ActionValue :type Boolean) (ElapsedSeconds :type "Float (double-precision)") (TriggeredSeconds :type "Float (double-precision)") (InputAction :type "InputAction Object Reference" :default "/Game/Exported/Inputs/Actions/IA_Drift.IA_Drift"))
  ;[1 1 1 1 30] Handle Inputs
  ;;[1 1 1] Handle Input Drift/MiniJump
  (:`Triggered`
    (if (not (`self.IsDrifting`))
      (if (== (`|GetInputActionValue`) 0.0)
        (if (`self.IsGrounded`)
          (`self.Jump`))
        (else
          (if (`self.IsGrounded`) :!label _label_3
            (`self.Drift` ElapsedSeconds))))
      (else
        (goto _label_3))))
  (:`Completed`
    (`self.End Drift`)
    (set `self.PrevDriftStrength` -1)))

(event `Jump`
  (bind _kartbody (`self.KartBody`))
  ;[1 1 1 1 30] Custom Events
  ;;[1 1 1] Mini Jump when not Steering Nor Drifting
  (if (not (`self.IsJumping`))
    (set `self.IsJumping` true)
    (`PrimitiveComponent.AddImpulse` _kartbody (* (`SceneComponent.GetUpVector` _kartbody) 250000.0) "None" false)
    (`KismetSystemLibrary.Delay` 0.6)
    (set `self.IsJumping` false)))

(event `Drift`
  (params (ElapsedTime :type "Float (double-precision)"))
  (bind _kartbody (`self.KartBody`))
  (bind _movementcomponent (`self.MovementComponent`))
  (bind _returnvalue (`SceneComponent.GetUpVector` _kartbody))
  ;[1 1 1 1 30] Custom Events
  ;;[1 1 1] Drift
  (if (not (`self.IsDrifting`))
    (set `self.IsDrifting` true)
    (`|ExecutionSequence`
      (:`then_0`
        ;;;[1 1 1] Activate Associated Particle Systems
        (`SceneComponent.SetHiddenInGame` (`self.DriftSparkParticle_L`) true false)
        (`SceneComponent.SetHiddenInGame` (`self.DriftSparkParticle_R`) true false)
        (`ActorComponent.Activate` (`self.DriftSmokeParticle_L`) false)
        (`ActorComponent.Activate` (`self.DriftSmokeParticle_R`) false)
        (`ActorComponent.Activate` (`self.DriftSparkParticle_L`) false)
        (`ActorComponent.Activate` (`self.DriftSparkParticle_R`) false))
      (:`then_1`
        ;;;[1 1 1] Apply Initial Drift Impulse
        (`PrimitiveComponent.AddImpulse` _kartbody (* _returnvalue 200000.0) "None" false)
        (`KismetSystemLibrary.Delay` 0.2)
        (`PrimitiveComponent.AddAngularImpulseInDegrees` _kartbody (* _returnvalue 1000000000.0 (`KismetMathLibrary.SelectInt` 1 -1 (> (`/Game/Exported/TanookiKart/Blueprints/BP_MovementComponent.CurrentAngularSpeed` (`self.MovementComponent`)) 0.0))) "None" false)
        (set `/Game/Exported/TanookiKart/Blueprints/BP_MovementComponent.TargetAngularSpeed` (* (`/Game/Exported/TanookiKart/Blueprints/BP_MovementComponent.TargetAngularSpeed` _movementcomponent) 0.2) _movementcomponent)))
    (else
      (`self.Set Drift Particle Color` ElapsedTime))))

(event `Boost`
  (params (BoostStrength :type "Float (double-precision)") (BoostTime :type "Float (double-precision)"))
  ;[1 1 1 1 30] Custom Events
  ;;[1 1 1] Boost
  (`|ExecutionSequence`
    (:`then_0`
      (set `self.BoostMultiplier` BoostStrength)
      (`ActorComponent.Activate` (`self.BoostParticle_L`) false)
      (`ActorComponent.Activate` (`self.BoostParticle_R`) false)
      (`ActorComponent.Activate` (`self.SpeedlinesParticle`) false)
      (bind (_direction _increasedfov) (`Timeline|Timeline_IncreaseFOV` :!via `PlayFromStart`)
        (:`Update`
          (`CameraComponent.SetFieldOfView` (`self.ChaseCamera`) _increasedfov))))
    (:`then_1`
      (`KismetSystemLibrary.Delay` BoostTime)
      (set `self.BoostMultiplier` 1.0)
      (`ActorComponent.Deactivate` (`self.BoostParticle_L`))
      (`ActorComponent.Deactivate` (`self.BoostParticle_R`))
      (`ActorComponent.Deactivate` (`self.SpeedlinesParticle`))
      (bind (_direction_2 _increasedfov_2 _decreasedfov) (`Timeline|Timeline_DecreaseFOV` :!via `PlayFromStart`)
        (:`Update`
          (`CameraComponent.SetFieldOfView` (`self.ChaseCamera`) _decreasedfov))))))

(event `self.SurfaceChecker.OnComponentBeginOverlap`
  (params (OverlappedComponent :type "PrimitiveComponent Object Reference") (OtherActor :type "Actor Object Reference") (OtherComp :type "PrimitiveComponent Object Reference") (OtherBodyIndex :type Integer) (bFromSweep :type Boolean) (SweepResult :type "HitResult Structure (by ref)"))
  (`KismetSystemLibrary.PrintString` (`KismetSystemLibrary.GetDisplayName` OverlappedComponent) true true (struct :`G` 1.0 :`B` 0.029682 :`A` 1.0) 1.0)
  (if (`ActorComponent.ComponentHasTag` OverlappedComponent "BoostPanel")
    (`KismetSystemLibrary.PrintString` "Boost" true false (struct :`G` 0.66 :`B` 1.0 :`A` 1.0) 1.0)
    (else
      (`KismetSystemLibrary.PrintString` "NoBoost" true false (struct :`R` 1.0 :`B` 0.126577 :`A` 1.0) 1.0))))

(fn `CheckIfGrounded`
  (for _index (range 4)
    (if (`/Game/Exported/TanookiKart/Blueprints/BP_HoverComponent.IsHit` (select `int` _index :`0` (`self.HoverComponent_FL`) :`1` (`self.HoverComponent_RL`) :`2` (`self.HoverComponent_RR`) :`3` (`self.HoverComponent_FR`)))
      (set `self.IsGrounded` true)
      (break)
      (else
        (set `self.IsGrounded` false)))))

(fn `End Drift`
  (bind _prevdriftstrength (`self.PrevDriftStrength`))
  (bind _output (`|GetArrayItem` (`self.DriftFxColors`)))
  (if (`self.IsDrifting`)
    (`|ExecutionSequence`
      (:`then_0`
        ;[1 1 1] Deactivate Particle Systems
        (`ActorComponent.Deactivate` (`self.DriftSmokeParticle_L`))
        (`ActorComponent.Deactivate` (`self.DriftSmokeParticle_R`))
        (`ActorComponent.Deactivate` (`self.DriftSparkParticle_L`))
        (`ActorComponent.Deactivate` (`self.DriftSparkParticle_R`)))
      (:`then_1`
        ;[1 1 1] Reset Particle Color
        (`FXSystemComponent.SetVectorParameter` (`self.DriftSparkParticle_L`) "SparkColor" _output)
        (`FXSystemComponent.SetVectorParameter` (`self.DriftSparkParticle_R`) "SparkColor" _output))
      (:`then_2`
        ;[1 1 1] Reset Variables
        (set `/Game/Exported/TanookiKart/Blueprints/BP_MovementComponent.TargetAngularSpeed` 0.0 (`self.MovementComponent`))
        (set `self.DriftStrength` -1)
        (set `self.IsDrifting` false))
      (:`then_3`
        ;[1 1 1] Apply Boost
        (if (<= 0 _prevdriftstrength)
          (`self.Boost` (select `int` _prevdriftstrength :`0` 1.5 :`1` 1.8 :`2` 2.2) (select `int` _prevdriftstrength :`0` 0.621 :`1` 1.647 :`2` 2.633)))))))

(fn `Set Drift Particle Color`
  (params (DriftTime :type "Float (double-precision)"))
  (bind _output (`|GetArrayItem` (`self.DriftFxColors`) (`self.DriftStrength`)))
  (bind _output_2 (`|GetArrayItem` (`self.DriftFxColors`) (`self.DriftStrength`)))
  (`|ExecutionSequence`
    (:`then_0`
      ;[1 1 1] Adjust Boost Level
      (if (>= DriftTime 5.0)
        (set `self.DriftStrength` 2)
        (elif (>= DriftTime 3.0)
          (set `self.DriftStrength` 1)
          (elif (>= DriftTime 1.7)
            (set `self.DriftStrength` 0)))))
    (:`then_1`
      ;[1 1 1] Play Drift Level Change Particle System
      (if (!= (`self.PrevDriftStrength`) (`self.DriftStrength`))
        (bind _returnvalue (`GameplayStatics.SpawnEmitterAttached` "/Game/Exported/Particles/PS_Shockwave.PS_Shockwave" (`self.Emitter_L`) "None" (31.0 -48.8 -27.0)))
        (bind _returnvalue_2 (`GameplayStatics.SpawnEmitterAttached` "/Game/Exported/Particles/PS_Shockwave.PS_Shockwave" (`self.Emitter_R`) "None" (32.7 49.1 -27.3)))
        (`FXSystemComponent.SetVectorParameter` _returnvalue_2 "Color" _output)
        (`FXSystemComponent.SetVectorParameter` _returnvalue "Color" _output))
      (set `self.PrevDriftStrength` (`self.DriftStrength`)))
    (:`then_2`
      ;[1 1 1] Adjust Drift Particle Visibility and Color
      (if (>= (`self.DriftStrength`) 0)
        (`SceneComponent.SetHiddenInGame` (`self.DriftSparkParticle_L`) false false)
        (`SceneComponent.SetHiddenInGame` (`self.DriftSparkParticle_R`) false false)
        (`ActorComponent.Deactivate` (`self.DriftSmokeParticle_L`))
        (`ActorComponent.Deactivate` (`self.DriftSmokeParticle_R`))
        (`FXSystemComponent.SetVectorParameter` (`self.DriftSparkParticle_L`) "SparkColor" _output_2)
        (`FXSystemComponent.SetVectorParameter` (`self.DriftSparkParticle_R`) "SparkColor" _output_2)))))

(fn `Set Steering Angle`
  (bind _maxsteeringangle (`self.MaxSteeringAngle`))
  (bind _maxsteeringangle_2 (`self.MaxSteeringAngle`))
  (bind _targetangularspeed (`/Game/Exported/TanookiKart/Blueprints/BP_MovementComponent.TargetAngularSpeed` (`self.MovementComponent`)))
  (if (`KismetMathLibrary.InRange_FloatFloat` _targetangularspeed -0.9 0.9)
    (set `self.SteeringAngle` (`KismetMathLibrary.FClamp` (* (`self.SteeringAngle`) 0.95) (* _maxsteeringangle_2 -1.0) _maxsteeringangle_2))
    (else
      (set `self.SteeringAngle` (`KismetMathLibrary.FClamp` (+ (`self.SteeringAngle`) (* 2.0 (`KismetMathLibrary.SelectFloat` 1.0 -1.0 (> _targetangularspeed 0.0)))) (* _maxsteeringangle -1.0) _maxsteeringangle))))
  (`SceneComponent.K2_SetRelativeRotation` (`self.WheelYaw_FR`) (`KismetMathLibrary.MakeRotator` 0.0 0.0 (`self.SteeringAngle`)) false false)
  (`SceneComponent.K2_SetRelativeRotation` (`self.WheelYaw_FL`) (`KismetMathLibrary.MakeRotator` 0.0 0.0 (`self.SteeringAngle`)) false false))

(fn `Set Wheel Rotation`
  (for _index (range 4)
    (`SceneComponent.K2_AddLocalRotation` (select `int` _index :`0` (`self.TanookiTires_FL`) :`1` (`self.TanookiTires_FR`) :`2` (`self.TanookiTires_RR`) :`3` (`self.TanookiTires_RL`)) (`KismetMathLibrary.MakeRotator` 0.0 (* (`KismetMathLibrary.RadiansToDegrees` (* (/ (`/Game/Exported/TanookiKart/Blueprints/BP_MovementComponent.CurrentSpeed` (`self.MovementComponent`)) (`/Game/Exported/TanookiKart/Blueprints/BP_HoverComponent.TireRadius` (`self.HoverComponent_FL`))) (`GameplayStatics.GetWorldDeltaSeconds`) 0.2)) -1.0)) false false)))

(fn `UserConstructionScript`)