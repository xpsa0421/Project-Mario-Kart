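; Player kart pawn for a kart racer, handling steering, throttle, drift, jump, boost, horn and camera toggle.
; Inputs set target speeds on a movement component, while Tick derives grounding from four hover traces and animates the wheels.
; Longer drifts raise a colour-coded tier that grants a boost on release.
; Holding throttle before the race charges a start boost, but overcharging explodes and briefly disables input.
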(event `self.ReceiveTick`
  (params (DeltaSeconds :type "Float (single-precision)"))
  (bind _lateralstabiliser (`self.LateralStabiliser`))
  ;[1 1 1] Alter Kart Wheel Animation and Status
  (`self.CheckIfGrounded`)
  (`self.Set Steering Angle`)
  (`self.Set Wheel Rotation`)
  (`KismetSystemLibrary.PrintString` (`KismetStringLibrary.Conv_BoolToString` (`self.IsGrounded`)) true true (struct :`G` 0.66 :`B` 1.0 :`A` 1.0) 0.0 :!enabledstate Disabled)
  (if (`self.IsGrounded`)
    (`ActorComponent.Activate` _lateralstabiliser false)
    (else
      (`ActorComponent.Deactivate` _lateralstabiliser))))

(event `self.ReceiveBeginPlay`
  ;[1 1 1 1 30] Initial Settings
  (`|ExecutionSequence`
    (:`then_0`
      ;;[1 1 1] Initialise Particle System Parameters
      (`FXSystemComponent.SetIntParameter` (`self.SmokeParticle_L`) "ParticleCount" 100)
      (`FXSystemComponent.SetIntParameter` (`self.SmokeParticle_R`) "ParticleCount" 100)
      (`FXSystemComponent.SetIntParameter` (`self.DriftSmokeParticle_L` :!enabledstate Disabled) "ParticleCount" 10000 :!enabledstate Disabled)
      (`FXSystemComponent.SetIntParameter` (`self.DriftSmokeParticle_R` :!enabledstate Disabled) "ParticleCount" 10000 :!enabledstate Disabled))
    (:`then_1`
      ;;[1 1 1] Set Default Camera
      (`ActorComponent.SetActive` (`self.ChaseCamera`) true false)
      (`ActorComponent.SetActive` (`self.RearCamera`) false false))
    (:`then_2`
      ;;[1 1 1] CineCamera Blend
      (`PlayerController.SetViewTargetWithBlend` (`GameplayStatics.GetPlayerController` 0) (`ChildActorComponent.ChildActor` (`self.CineCameraActor`)) 0.0 "VTBlend_EaseInOut" 0.0 false)
      (`KismetSystemLibrary.Delay` 2.0)
      (`PlayerController.SetViewTargetWithBlend` (`GameplayStatics.GetPlayerController` 0) self 2.0 "VTBlend_Linear" 0.0 false))))

(event `EnhancedInput|/Game/Exported/Inputs/Actions/IA_Steer`
  (params (ActionValue :type "Float (double-precision)") (ElapsedSeconds :type "Float (double-precision)") (TriggeredSeconds :type "Float (double-precision)") (InputAction :type "InputAction Object Reference" :default "/Game/Exported/Inputs/Actions/IA_Steer.IA_Steer"))
  (bind _returnvalue (`|GetInputActionValue`))
  ;[1 1 1 1 30] Handle Inputs
  ;;[1 1 1] Handle Input Steer
  (:`Triggered`
    (if (`self.IsRacing`) :!label _label
      (if (not (`self.IsDrifting`))
        (set `/Game/Exported/TanookiKart/Blueprints/BP_MovementComponent.TargetAngularSpeed` (* ActionValue 100.0 (select `bool` (== _returnvalue 0.0) :`false` _returnvalue :`true` 1.0)) (`self.MovementComponent`)))))
  (:`Completed`
    (goto _label)))

(event `EnhancedInput|/Game/Exported/Inputs/Actions/IA_Throttle`
  (params (ActionValue :type "Float (double-precision)") (ElapsedSeconds :type "Float (double-precision)") (TriggeredSeconds :type "Float (double-precision)") (InputAction :type "InputAction Object Reference" :default "/Game/Exported/Inputs/Actions/IA_Throttle.IA_Throttle"))
  (bind _returnvalue (* ElapsedSeconds 1.3))
  (bind _returnvalue_2 (`KismetMathLibrary.FTrunc` (* ElapsedSeconds 320.0)))
  ;[1 1 1 1 30] Handle Inputs
  ;;[1 1 1] Handle Input Throttle
  (:`Triggered`
    (if (`self.IsRacing`)
      (`AudioParameterControllerInterface.SetIntParameter` (`self.Sounds`) "CarState" 2)
      (if (`self.IsCharging`)
        ;;;[1 1 1] Apply Boost or Explosion Depending on Charge Time
        (if (> ElapsedSeconds 2.1)
          (`self.ChargeFail`)
          (else
            (`self.Boost` _returnvalue _returnvalue)
            (`ActorComponent.Deactivate` (`self.SmokeParticle_L`))
            (`ActorComponent.Deactivate` (`self.SmokeParticle_R`))
            (`self.AddLinearVelocity` ActionValue)
            (set `self.IsCharging` false)))
        (else
          (`self.AddLinearVelocity` ActionValue :!label _label_2)))
      (elif (`self.IsCharging`)
        ;;;[1 1 1] Update Charging Particle Emitters
        (if (> ElapsedSeconds 2.1)
          (`self.ChargeFail`)
          (else
            (`FXSystemComponent.SetIntParameter` (`self.SmokeParticle_L`) "ParticleCount" _returnvalue_2)
            (`FXSystemComponent.SetIntParameter` (`self.SmokeParticle_R`) "ParticleCount" _returnvalue_2)))
        (else
          ;;;[1 1 1] Activate Charging Particle Emitters
          (set `self.IsCharging` true)
          (`ActorComponent.Activate` (`self.SmokeParticle_L`) false)
          (`ActorComponent.Activate` (`self.SmokeParticle_R`) false)
          (`AudioParameterControllerInterface.SetIntParameter` (`self.Sounds`) "CarState" 1)))))
  (:`Completed`
    (if (`self.IsRacing`)
      (goto _label_2)
      (else
        ;;;[1 1 1] Deactivate Charging Particle Emitters
        (`ActorComponent.Deactivate` (`self.SmokeParticle_L`))
        (`ActorComponent.Deactivate` (`self.SmokeParticle_R`))
        (set `self.IsCharging` false)))))

(event `EnhancedInput|/Game/Exported/Inputs/Actions/IA_Horn`
  (params (ActionValue :type Boolean) (ElapsedSeconds :type "Float (double-precision)") (TriggeredSeconds :type "Float (double-precision)") (InputAction :type "InputAction Object Reference" :default "/Game/Exported/Inputs/Actions/IA_Horn.IA_Horn"))
  ;[1 1 1 1 30] Handle Inputs
  ;;[1 1 1] Handle Input Horn
  (:`Triggered`
    (if (not (`self.HornPlaying`))
      (set `self.HornPlaying` true)
      (`GameplayStatics.PlaySoundAtLocation` "/Game/Exported/Sounds/Karts/WAV_Tnk_Horn.WAV_Tnk_Horn" (`self.K2_GetActorLocation`) (struct) 0.8 1.0 0.0 null null null null)
      (`KismetSystemLibrary.Delay` 0.531)
      (set `self.HornPlaying` false))))

(event `EnhancedInput|/Game/Exported/Inputs/Actions/IA_Boost`
  (params (ActionValue :type Boolean) (ElapsedSeconds :type "Float (double-precision)") (TriggeredSeconds :type "Float (double-precision)") (InputAction :type "InputAction Object Reference" :default "/Game/Exported/Inputs/Actions/IA_Boost.IA_Boost"))
  ;[1 1 1 1 30] Handle Inputs
  ;;[1 1 1] Handle Input Boost
  (:`Triggered`
    (if (and (`self.IsRacing`) (!= (`self.BoosterCount`) 0) (== (`self.BoostMultiplier`) 1.0))
      (`/Engine/EditorBlueprintResources/StandardMacros.DecrementInt` (`self.BoosterCount`)
        (:`  `
          (bind _asbp_kart_controller (cast `/Game/Exported/Inputs/BP_KartController` (`self.GetController`)))
          (`/Engine/EditorBlueprintResources/StandardMacros.DecrementInt` (`/Game/UI/InGame/WBP_InGame.BoosterCount` (`/Game/Exported/Inputs/BP_KartController.InGameUI` _asbp_kart_controller))
            (:`  `
              (`self.Boost` 1.6 2.0))))))))

(event `EnhancedInput|/Game/Exported/Inputs/Actions/IA_Drift`
  (params (ActionValue :type Boolean) (ElapsedSeconds :type "Float (double-precision)") (TriggeredSeconds :type "Float (double-precision)") (InputAction :type "InputAction Object Reference" :default "/Game/Exported/Inputs/Actions/IA_Drift.IA_Drift"))
  (bind _isracing (`self.IsRacing`))
  ;[1 1 1 1 30] Handle Inputs
  ;;[1 1 1] Handle Input Drift/MiniJump
  (:`Triggered`
    (if _isracing
      (if (not (`self.IsDrifting`))
        (if (== (`|GetInputActionValue`) 0.0)
          (if (`self.IsGrounded`)
            (`self.Jump`))
          (else
            (if (`self.IsGrounded`) :!label _label_3
              (`self.Drift` ElapsedSeconds))))
        (else
          (goto _label_3)))))
  (:`Completed`
    (if _isracing
      (`self.End Drift`)
      (set `self.PrevDriftStrength` -1))))

(event `EnhancedInput|/Game/Exported/Inputs/Actions/IA_ToggleCamera`
  (params (ActionValue :type Boolean) (ElapsedSeconds :type "Float (double-precision)") (TriggeredSeconds :type "Float (double-precision)") (InputAction :type "InputAction Object Reference" :default "/Game/Exported/Inputs/Actions/IA_ToggleCamera.IA_ToggleCamera"))
  ;[1 1 1 1 30] Handle Inputs
  ;;[1 1 1] Handle Input Toggle Camera
  (:`Triggered`
    (if (`self.IsRacing`)
      (`/Engine/EditorBlueprintResources/StandardMacros.FlipFlop`
        (:`A`
          (`ActorComponent.SetActive` (`self.ChaseCamera`) false false)
          (`ActorComponent.SetActive` (`self.RearCamera`) true false))
        (:`B`
          (`ActorComponent.SetActive` (`self.ChaseCamera`) true false)
          (`ActorComponent.SetActive` (`self.RearCamera`) false false))))))

(event `Jump`
  (bind _kartbody (`self.KartBody`))
  ;[1 1 1 1 30] Custom Events
  ;;[1 1 1] Mini Jump when not Steering Nor Drifting
  (if (not (`self.IsJumping`))
    (set `self.IsJumping` true)
    (`PrimitiveComponent.AddImpulse` _kartbody (* (`SceneComponent.GetUpVector` _kartbody) 250000.0) "None" false)
    (`KismetSystemLibrary.Delay` 0.6)
    (set `self.IsJumping` false)))

(event `Drift`
  (params (ElapsedTime :type "Float (double-precision)"))
  (bind _kartbody (`self.KartBody`))
  (bind _movementcomponent (`self.MovementComponent`))
  (bind _returnvalue (`SceneComponent.GetUpVector` _kartbody))
  ;[1 1 1 1 30] Custom Events
  ;;[1 1 1] Drift
  (if (not (`self.IsDrifting`))
    (set `self.IsDrifting` true)
    (`|ExecutionSequence`
      (:`then_0`
        ;;;[1 1 1] Activate Associated Particle Systems
        (`SceneComponent.SetHiddenInGame` (`self.DriftSparkParticle_L`) true false)
        (`SceneComponent.SetHiddenInGame` (`self.DriftSparkParticle_R`) true false)
        (`ActorComponent.Activate` (`self.DriftSmokeParticle_L`) false)
        (`ActorComponent.Activate` (`self.DriftSmokeParticle_R`) false)
        (`ActorComponent.Activate` (`self.DriftSparkParticle_L`) false)
        (`ActorComponent.Activate` (`self.DriftSparkParticle_R`) false))
      (:`then_1`
        ;;;[1 1 1] Apply Initial Drift Impulse
        (`PrimitiveComponent.AddImpulse` _kartbody (* _returnvalue 200000.0) "None" false)
        (`KismetSystemLibrary.Delay` 0.2)
        (`PrimitiveComponent.AddAngularImpulseInDegrees` _kartbody (* _returnvalue 1000000000.0 (`KismetMathLibrary.SelectInt` 1 -1 (> (`/Game/Exported/TanookiKart/Blueprints/BP_MovementComponent.CurrentAngularSpeed` (`self.MovementComponent`)) 0.0))) "None" false)
        (set `/Game/Exported/TanookiKart/Blueprints/BP_MovementComponent.TargetAngularSpeed` (* (`/Game/Exported/TanookiKart/Blueprints/BP_MovementComponent.TargetAngularSpeed` _movementcomponent) 0.3) _movementcomponent)))
    (else
      (`self.UpdateDriftParticles` ElapsedTime))))

(event `Boost`
  (params (BoostStrength :type "Float (double-precision)") (BoostTime :type "Float (double-precision)"))
  ;[1 1 1 1 30] Custom Events
  ;;[1 1 1] Boost
  (`AudioComponent.SetIntParameter` (`self.Sounds`) "CarState" 3)
  (`|ExecutionSequence`
    (:`then_0`
      (set `self.BoostMultiplier` BoostStrength)
      (`ActorComponent.Activate` (`self.BoostParticle_L`) false)
      (`ActorComponent.Activate` (`self.BoostParticle_R`) false)
      (`ActorComponent.Activate` (`self.SpeedlinesParticle`) false)
      (bind (_direction _increasedfov) (`Timeline|Timeline_IncreaseFOV` :!via `PlayFromStart`)
        (:`Update`
          (`CameraComponent.SetFieldOfView` (`self.ChaseCamera`) _increasedfov))))
    (:`then_1`
      (`KismetSystemLibrary.Delay` BoostTime)
      (set `self.BoostMultiplier` 1.0)
      (`ActorComponent.Deactivate` (`self.BoostParticle_L`))
      (`ActorComponent.Deactivate` (`self.BoostParticle_R`))
      (`ActorComponent.Deactivate` (`self.SpeedlinesParticle`))
      (bind (_direction_2 _increasedfov_2 _decreasedfov) (`Timeline|Timeline_DecreaseFOV` :!via `PlayFromStart`)
        (:`Update`
          (`CameraComponent.SetFieldOfView` (`self.ChaseCamera`) _decreasedfov)
          (`AudioComponent.SetIntParameter` (`self.Sounds`) "CarState" 2))))))

(event `ChargeFail`
  ;[1 1 1 1 30] Custom Events
  ;;[1 1 1] Spawn Emitter and Disable Input Upon Charge Fail
  (set `self.IsCharging` false)
  (`GameplayStatics.PlaySound2D` "/Game/StarterContent/Audio/Explosion01.Explosion01" 1.0 1.0 0.0 null null)
  (`GameplayStatics.SpawnEmitterAtLocation` "/Game/StarterContent/Particles/P_Explosion.P_Explosion" (`self.K2_GetActorLocation`))
  (`ActorComponent.Deactivate` (`self.SmokeParticle_L`))
  (`ActorComponent.Deactivate` (`self.SmokeParticle_R`))
  (`self.DisableInput` null)
  (`KismetSystemLibrary.Delay` 1.5)
  (`self.EnableInput` null))

(event `Glide`)

(fn `AddLinearVelocity`
  (params (Direction :type "Float (double-precision)"))
  (if (`self.IsGrounded`)
    (set `/Game/Exported/TanookiKart/Blueprints/BP_MovementComponent.TargetSpeed` (* Direction (`self.DefaultSpeedMultiplier`) (`self.BoostMultiplier`)) (`self.MovementComponent`))))

(fn `CheckIfGrounded`
  (set `self.NumTyreOnGround` 0)
  (set `self.IsGrounded` false)
  (for _index (range 4)
    (if (`/Game/Exported/TanookiKart/Blueprints/BP_HoverComponent.TraceHit` (select `int` _index :`0` (`self.HoverComponent_FL`) :`1` (`self.HoverComponent_RL`) :`2` (`self.HoverComponent_RR`) :`3` (`self.HoverComponent_FR`)))
      (bind _result (`/Engine/EditorBlueprintResources/StandardMacros.IncrementInt` (`self.NumTyreOnGround`))
        (:`  `
          (if (== _result 2)
            (set `self.IsGrounded` true)
            (break)))))))

(fn `End Drift`
  (bind _prevdriftstrength (`self.PrevDriftStrength`))
  (bind _output (`|GetArrayItem` (`self.DriftFxColors`)))
  (if (`self.IsDrifting`)
    (`|ExecutionSequence`
      (:`then_0`
        ;[1 1 1] Deactivate Particle Systems
        (`ActorComponent.Deactivate` (`self.DriftSmokeParticle_L`))
        (`ActorComponent.Deactivate` (`self.DriftSmokeParticle_R`))
        (`ActorComponent.Deactivate` (`self.DriftSparkParticle_L`))
        (`ActorComponent.Deactivate` (`self.DriftSparkParticle_R`)))
      (:`then_1`
        ;[1 1 1] Reset Particle Color
        (`FXSystemComponent.SetVectorParameter` (`self.DriftSparkParticle_L`) "SparkColor" _output)
        (`FXSystemComponent.SetVectorParameter` (`self.DriftSparkParticle_R`) "SparkColor" _output))
      (:`then_2`
        ;[1 1 1] Reset Variables
        (set `/Game/Exported/TanookiKart/Blueprints/BP_MovementComponent.TargetAngularSpeed` 0.0 (`self.MovementComponent`))
        (set `self.DriftStrength` -1)
        (set `self.IsDrifting` false))
      (:`then_3`
        ;[1 1 1] Apply Boost
        (if (<= 0 _prevdriftstrength)
          (`self.Boost` (select `int` _prevdriftstrength :`0` 1.5 :`1` 1.8 :`2` 2.2) (select `int` _prevdriftstrength :`0` 0.621 :`1` 1.647 :`2` 2.633)))))))

(fn `Set Steering Angle`
  (bind _maxsteeringangle (`self.MaxSteeringAngle`))
  (bind _maxsteeringangle_2 (`self.MaxSteeringAngle`))
  (bind _targetangularspeed (`/Game/Exported/TanookiKart/Blueprints/BP_MovementComponent.TargetAngularSpeed` (`self.MovementComponent`)))
  (if (`KismetMathLibrary.InRange_FloatFloat` _targetangularspeed -0.9 0.9)
    (set `self.SteeringAngle` (`KismetMathLibrary.FClamp` (* (`self.SteeringAngle`) 0.95) (* _maxsteeringangle_2 -1.0) _maxsteeringangle_2))
    (else
      (set `self.SteeringAngle` (`KismetMathLibrary.FClamp` (+ (`self.SteeringAngle`) (* 2.0 (`KismetMathLibrary.SelectFloat` 1.0 -1.0 (> _targetangularspeed 0.0)))) (* _maxsteeringangle -1.0) _maxsteeringangle))))
  (`SceneComponent.K2_SetRelativeRotation` (`self.WheelYaw_FR`) (`KismetMathLibrary.MakeRotator` 0.0 0.0 (`self.SteeringAngle`)) false false)
  (`SceneComponent.K2_SetRelativeRotation` (`self.WheelYaw_FL`) (`KismetMathLibrary.MakeRotator` 0.0 0.0 (`self.SteeringAngle`)) false false))

(fn `Set Wheel Rotation`
  (for _index (range 4)
    (`SceneComponent.K2_AddLocalRotation` (select `int` _index :`0` (`self.TanookiTires_FL`) :`1` (`self.TanookiTires_FR`) :`2` (`self.TanookiTires_RR`) :`3` (`self.TanookiTires_RL`)) (`KismetMathLibrary.MakeRotator` 0.0 (* (`KismetMathLibrary.RadiansToDegrees` (* (/ (`/Game/Exported/TanookiKart/Blueprints/BP_MovementComponent.CurrentSpeed` (`self.MovementComponent`)) (`/Game/Exported/TanookiKart/Blueprints/BP_HoverComponent.TireRadius` (`self.HoverComponent_FL`))) (`GameplayStatics.GetWorldDeltaSeconds`) 0.2)) -1.0)) false false)))

(fn `ToggleHeadLight`
  (bind _islighton (`self.IsLightOn`))
  (set `self.IsLightOn` (not (`self.IsLightOn`)))
  (`|ExecutionSequence`
    (:`then_0`
      ;[1 1 1] Change Material
      (if (`self.IsLightOn`)
        (if (== (`self.BoostMultiplier`) 1.0)
          (`PrimitiveComponent.SetMaterial` (`self.KartBody`) 1 "/Game/Exported/TanookiKart/Materials/M_KartTanooki_Body_HeadLight.M_KartTanooki_Body_HeadLight"))
        (elif (== (`self.BoostMultiplier`) 1.0)
          (`PrimitiveComponent.SetMaterial` (`self.KartBody`) 1 "/Game/Exported/TanookiKart/Materials/M_KartTanooki_Body_Default.M_KartTanooki_Body_Default"))))
    (:`then_1`
      ;[1 1 1] Turn On/Off Light
      (`SceneComponent.SetVisibility` (`self.HeadLight_L`) _islighton false)
      (`SceneComponent.SetVisibility` (`self.HeadLight_R`) _islighton false))))

(fn `UpdateDriftParticles`
  (params (DriftTime :type "Float (double-precision)"))
  (bind _output (`|GetArrayItem` (`self.DriftFxColors`) (`self.DriftStrength`)))
  (bind _output_2 (`|GetArrayItem` (`self.DriftFxColors`) (`self.DriftStrength`)))
  (`|ExecutionSequence`
    (:`then_0`
      ;[1 1 1] Adjust Boost Level
      (if (>= DriftTime 2.6)
        (set `self.DriftStrength` 2)
        (elif (>= DriftTime 2.0)
          (set `self.DriftStrength` 1)
          (elif (>= DriftTime 1.3)
            (set `self.DriftStrength` 0)))))
    (:`then_1`
      ;[1 1 1] Play Drift Level Change Particle System
      (if (!= (`self.PrevDriftStrength`) (`self.DriftStrength`))
        (bind _returnvalue (`GameplayStatics.SpawnEmitterAttached` "/Game/Exported/Particles/PS_Shockwave.PS_Shockwave" (`self.Emitter_L`) "None" (13.3 -24.0 -10.0)))
        (bind _returnvalue_2 (`GameplayStatics.SpawnEmitterAttached` "/Game/Exported/Particles/PS_Shockwave.PS_Shockwave" (`self.Emitter_R`) "None" (13.3 24.0 -10.0)))
        (`FXSystemComponent.SetVectorParameter` _returnvalue_2 "Color" _output)
        (`FXSystemComponent.SetVectorParameter` _returnvalue "Color" _output))
      (set `self.PrevDriftStrength` (`self.DriftStrength`)))
    (:`then_2`
      ;[1 1 1] Adjust Drift Particle Visibility and Color
      (if (>= (`self.DriftStrength`) 0)
        (`SceneComponent.SetHiddenInGame` (`self.DriftSparkParticle_L`) false false)
        (`SceneComponent.SetHiddenInGame` (`self.DriftSparkParticle_R`) false false)
        (`ActorComponent.Deactivate` (`self.DriftSmokeParticle_L`))
        (`ActorComponent.Deactivate` (`self.DriftSmokeParticle_R`))
        (`FXSystemComponent.SetVectorParameter` (`self.DriftSparkParticle_L`) "SparkColor" _output_2)
        (`FXSystemComponent.SetVectorParameter` (`self.DriftSparkParticle_R`) "SparkColor" _output_2)))))

(fn `UserConstructionScript`)