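; Scene component that acts as one raycast suspension point, pushing a physics-simulated owner up from the surface and positioning a tire mesh.
; Each tick it traces down its up vector to HoverDistance, then applies a spring-damper force at its location from normalised compression and its rate of change.
; The hit point also sets the tire's relative Z, using the child or grandchild mesh found at BeginPlay.
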(event `self.ReceiveBeginPlay`
  (`self.InitialiseParent`)
  (`self.InitialiseChildren`))

(event `self.ReceiveTick`
  (params (DeltaSeconds :type "Float (single-precision)"))
  (`self.RefToBody`
    (:`then`
      (bind (_hitresult _is_hit) (`self.Trace Surface`))
      (if _is_hit
        (bind (_bblockinghit _binitialoverlap _time _distance _location) (`GameplayStatics.BreakHitResult` _hitresult))
        (`self.Update Suspension Force` _distance)
        (`self.Apply Suspension Force`)
        (`self.Update Tire Position` _location)))
    (:`else`)))

(fn `Apply Suspension Force`
  (if (`self.TraceHit`)
    (`PrimitiveComponent.AddForceAtLocation` (`self.RefToBody`) (* (`self.GetUpVector`) (`self.HoverForce`)) (`self.K2_GetComponentLocation`) "None")
    (`KismetSystemLibrary.PrintString` (`KismetStringLibrary.Concat_StrStr` (`KismetSystemLibrary.GetDisplayName` self) ": Add Force") true false (struct :`R` 0.264037 :`G` 0.765625 :`B` 0.150237 :`A` 1.0) (`GameplayStatics.GetWorldDeltaSeconds`) :!enabledstate Disabled)
    (return)
    (else
      (`KismetSystemLibrary.PrintString` (`KismetStringLibrary.Concat_StrStr` (`KismetSystemLibrary.GetDisplayName` self) ": No Force") true false (struct :`R` 0.765625 :`G` 0.039876 :`B` 0.313482 :`A` 1.0) (`GameplayStatics.GetWorldDeltaSeconds`) :!enabledstate Disabled))))

(fn `InitialiseChildren`
  (bind _returnvalue (`self.GetChildComponent` 0))
  (bind _returnvalue_2 (`self.GetChildComponent` _returnvalue 0))
  (`/Engine/EditorBlueprintResources/StandardMacros.IsValid` _returnvalue_2
    (:`Is Valid`
      (bind _asstatic_mesh_component (cast `StaticMeshComponent` _returnvalue_2))
      (set `self.RefToTire` _asstatic_mesh_component))
    (:`Is Not Valid`
      (bind _asstatic_mesh_component_2 (cast `StaticMeshComponent` _returnvalue))
      (set `self.RefToTire` _asstatic_mesh_component_2))))

(fn `InitialiseParent`
  (bind _asprimitive_component (cast `PrimitiveComponent` (`Actor.RootComponent` (`self.GetOwner`))))
  (bind _output_get (set `self.RefToBody` _asprimitive_component))
  (if (not (`self.IsSimulatingPhysics` _output_get "None"))
    (set `self.RefToBody` null))
  (return))

(fn `Trace Surface`
  (returns (HitResult :type "HitResult Structure") (`Is Hit` :type Boolean))
  (bind _returnvalue (`self.K2_GetComponentLocation`))
  (bind (_outhit _returnvalue_2) (`KismetSystemLibrary.LineTraceSingle` _returnvalue (- _returnvalue (* (`self.GetUpVector`) (`self.HoverDistance`))) "TraceTypeQuery1" false (`|MakeArray` (`self.GetOwner`)) "ForOneFrame"))
  (bind _output_get (set `self.TraceHit` _returnvalue_2))
  (return _outhit _output_get))

(fn `Update Suspension Force`
  (params (`Hit Distance` :type "Float (double-precision)"))
  (bind _hoverdistance (`self.HoverDistance`))
  (bind _returnvalue (/ (- _hoverdistance (`local.Hit Distance`)) _hoverdistance))
  (bind _output_get (set `self.HoverForce` (+ (* (/ (- _returnvalue (`self.PrevCompression`)) (`GameplayStatics.GetWorldDeltaSeconds`)) (`self.Damping`)) (* _returnvalue (`self.Stiffness`)))))
  (`KismetSystemLibrary.PrintString` (`KismetStringLibrary.Conv_DoubleToString` _output_get) true true (struct :`G` 0.66 :`B` 1.0 :`A` 1.0) (`GameplayStatics.GetWorldDeltaSeconds`) :!enabledstate Disabled)
  (set `self.PrevCompression` _returnvalue)
  (return))

(fn `Update Tire Position`
  (params (HitLocation :type "Vector Structure"))
  (`self.K2_SetRelativeLocation` (`self.RefToTire`) (`KismetMathLibrary.MakeVector` 0.0 0.0 (`KismetMathLibrary.VSize` (- (+ HitLocation (* (`self.TireRadius`) (`self.GetUpVector`))) (`self.K2_GetComponentLocation`)))) false false)
  (return))