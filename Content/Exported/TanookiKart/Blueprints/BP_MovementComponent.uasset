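; Movement component for TanookiKart that drives a physics-simulated body toward target linear and angular speeds.
; On BeginPlay it caches the owner's root primitive component as the body.
; Each Tick it projects velocity onto the forward and up axes, then applies force and torque proportional to each speed error.
; This proportional control leaves the target values to be set outside the component.
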(event `self.ReceiveBeginPlay`
  (bind _asprimitive_component (cast `PrimitiveComponent` (`Actor.RootComponent` (`self.GetOwner`))))
  (set `self.RefToBody` _asprimitive_component))

(event `self.ReceiveTick`
  (params (DeltaSeconds :type "Float (single-precision)"))
  (`self.RefToBody`
    (:`then`
      (`self.UpdateLinearSpeed`)
      (`self.UpdateAngularSpeed`))
    (:`else`)))

(fn `UpdateAngularSpeed`
  (bind _reftobody (`self.RefToBody`))
  (bind _reftobody_2 (`self.RefToBody`))
  (set `self.CurrentAngularSpeed` (`KismetMathLibrary.Dot_VectorVector` (`PrimitiveComponent.GetPhysicsAngularVelocityInDegrees` _reftobody "None") (`SceneComponent.GetUpVector` _reftobody)))
  (`PrimitiveComponent.AddTorqueInDegrees` _reftobody_2 (* (`SceneComponent.GetUpVector` _reftobody_2) (* (- (`self.TargetAngularSpeed`) (`self.CurrentAngularSpeed`)) (`self.AngularSpeedToTorqueFactor`))) "None" false))

(fn `UpdateLinearSpeed`
  (bind _reftobody (`self.RefToBody`))
  (bind _reftobody_2 (`self.RefToBody`))
  (bind _returnvalue (`PrimitiveComponent.GetPhysicsLinearVelocity` _reftobody_2 "None"))
  (set `self.CurrentSpeed` (`KismetMathLibrary.Dot_VectorVector` _returnvalue (`SceneComponent.GetForwardVector` _reftobody_2)))
  (`PrimitiveComponent.AddForce` _reftobody (* (`SceneComponent.GetForwardVector` _reftobody) (* (- (`self.TargetSpeed`) (`self.CurrentSpeed`)) (`self.SpeedToForceFactor`))) "None" false))